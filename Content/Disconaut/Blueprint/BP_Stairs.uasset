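; BP_Stairs is an interactable staircase that teleports the player's BP_Disconaut pawn between two floors.
; On Interract, it checks and flips the pawn's IsFirstFloor flag to choose an upward or downward vertical offset.
; It then moves the pawn's capsule to a hardcoded X/Y position, applying that offset to its current height.
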(event EventBeginPlay)

(event Collision|EventActorBeginOverlap
  (params (OtherActor :type Actor%20Object%20Reference)))

(event EventTick
  (params (DeltaSeconds :type Float%20%28single-precision%29)))

(event EventInterract
  (bind _asbp_disconaut (Utilities|Casting|CastToBP_Disconaut (Game|Player|GetPlayerPawn 0)))
  (if (Variables|/Game/Disconaut/Blueprint/Character/BP_Disconaut.BP_Disconaut_C|GetIsFirstFloor _asbp_disconaut)
    (Variables|Default|SetTP_Length 3.4e+02)
    (Variables|/Game/Disconaut/Blueprint/Character/BP_Disconaut.BP_Disconaut_C|SetIsFirstFloor _asbp_disconaut false)
    (else
      (Variables|Default|SetTP_Length -3.4e+02)
      (Variables|/Game/Disconaut/Blueprint/Character/BP_Disconaut.BP_Disconaut_C|SetIsFirstFloor _asbp_disconaut true)))
  (Transformation|SetWorldLocation (Variables|/Script/Engine.Character|GetCapsuleComponent _asbp_disconaut) (Math|Vector|MakeVector 2.54e+03 945.0 (+ (.z (Transformation|GetWorldLocation (Variables|/Script/Engine.Character|GetCapsuleComponent _asbp_disconaut))) (Variables|Default|GetTP_Length))) false false))

(fn ConstructionScript)