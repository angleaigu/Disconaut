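; BP_ToiletCam is an interactable camera actor that takes over the player's view in Disconaut.
; Interract registers it as the Disconaut pawn's current look target, flags the pawn as looking, disables its movement and look, and blends the view to this actor over one second.
; Out restores movement and look, clears the looking flag and blends the view back to the pawn.
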(event EventBeginPlay)

(event Collision|EventActorBeginOverlap
  (params (OtherActor :type Actor%20Object%20Reference)))

(event EventTick
  (params (DeltaSeconds :type Float%20%28single-precision%29)))

(event EventInterract
  (bind _asbp_disconaut (Utilities|Casting|CastToBP_Disconaut (Game|Player|GetPlayerPawn 0)))
  (Variables|/Game/Disconaut/Blueprint/Character/BP_Disconaut.BP_Disconaut_C|SetActualLook _asbp_disconaut self)
  (Variables|/Game/Disconaut/Blueprint/Character/BP_Disconaut.BP_Disconaut_C|SetIsLooking _asbp_disconaut true)
  (Variables|/Game/Disconaut/Blueprint/Character/BP_Disconaut.BP_Disconaut_C|SetCanMoove _asbp_disconaut false)
  (Variables|/Game/Disconaut/Blueprint/Character/BP_Disconaut.BP_Disconaut_C|SetCanLook _asbp_disconaut false)
  (Game|Player|SetViewTargetwithBlend (Game|GetPlayerController 0) self 1.0 "VTBlend_Linear" 0.0 false))

(event EventOut
  (bind _asbp_disconaut (Utilities|Casting|CastToBP_Disconaut (Game|Player|GetPlayerPawn 0)))
  (Variables|/Game/Disconaut/Blueprint/Character/BP_Disconaut.BP_Disconaut_C|SetCanMoove _asbp_disconaut true)
  (Variables|/Game/Disconaut/Blueprint/Character/BP_Disconaut.BP_Disconaut_C|SetIsLooking _asbp_disconaut false)
  (Variables|/Game/Disconaut/Blueprint/Character/BP_Disconaut.BP_Disconaut_C|SetCanLook _asbp_disconaut true)
  (Game|Player|SetViewTargetwithBlend (Game|GetPlayerController 0) _asbp_disconaut 1.0 "VTBlend_Linear" 0.0 false))

(fn ConstructionScript)