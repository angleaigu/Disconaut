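; BP_Drink is an interactable drink that takes over the player's view and control when used.
; Interract flags BP_Disconaut as looking at it, locks movement and look, blends the camera to the drink, shows the cursor, then calls PossessPawn after a delay.
; IA_Cancel restores the player's state, blends the view back and re-possesses the Disconaut after a delay.
; IA_Fart only prints a debug string.
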(event Input|EnhancedActionEvents|EnhancedInputActionIA_Fart
  (params (ActionValue :type Boolean) (ElapsedSeconds :type Float%20%28double-precision%29) (TriggeredSeconds :type Float%20%28double-precision%29) (InputAction :type Input%20Action%20Object%20Reference :default "/Game/Disconaut/Input/Actions/IA_Fart.IA_Fart"))
  (Development|PrintString "poupou"))

(event Input|EnhancedActionEvents|EnhancedInputActionIA_Cancel
  (params (ActionValue :type Boolean) (ElapsedSeconds :type Float%20%28double-precision%29) (TriggeredSeconds :type Float%20%28double-precision%29) (InputAction :type Input%20Action%20Object%20Reference :default "/Game/Disconaut/Input/Actions/IA_Cancel.IA_Cancel"))
  (bind _returnvalue (Game|GetPlayerController 0))
  (Variables|/Game/Disconaut/Blueprint/Character/BP_Disconaut.BP_Disconaut_C|SetCanMoove (stale EventInterract _asbp_disconaut) true)
  (Variables|/Game/Disconaut/Blueprint/Character/BP_Disconaut.BP_Disconaut_C|SetIsLooking (stale EventInterract _asbp_disconaut) false)
  (Variables|/Game/Disconaut/Blueprint/Character/BP_Disconaut.BP_Disconaut_C|SetCanLook (stale EventInterract _asbp_disconaut) true)
  (Game|Player|SetViewTargetwithBlend _returnvalue (stale EventInterract _asbp_disconaut) 1.0 "VTBlend_Linear" 0.0 false)
  (Variables|/Script/Engine.PlayerController|SetbShowMouseCursor _returnvalue false)
  (Utilities|FlowControl|Delay 1.2)
  (Pawn|Possess (Game|GetPlayerController 0) (stale EventInterract _asbp_disconaut)))

(event EventBeginPlay)

(event Collision|EventActorBeginOverlap
  (params (OtherActor :type Actor%20Object%20Reference)))

(event EventTick
  (params (DeltaSeconds :type Float%20%28single-precision%29)))

(event EventInterract
  (bind _returnvalue (Game|GetPlayerController 0))
  ;[1 1 1] Get Camera and get possessed
  (bind _asbp_disconaut (Utilities|Casting|CastToBP_Disconaut (Game|Player|GetPlayerPawn 0)))
  (Variables|/Game/Disconaut/Blueprint/Character/BP_Disconaut.BP_Disconaut_C|SetActualLook _asbp_disconaut self)
  (Variables|/Game/Disconaut/Blueprint/Character/BP_Disconaut.BP_Disconaut_C|SetIsLooking _asbp_disconaut true)
  (Variables|/Game/Disconaut/Blueprint/Character/BP_Disconaut.BP_Disconaut_C|SetCanMoove _asbp_disconaut false)
  (Variables|/Game/Disconaut/Blueprint/Character/BP_Disconaut.BP_Disconaut_C|SetCanLook _asbp_disconaut false)
  (Game|Player|SetViewTargetwithBlend _returnvalue self 1.0 "VTBlend_Linear" 0.0 false)
  (Variables|/Script/Engine.PlayerController|SetbShowMouseCursor _returnvalue true)
  (Utilities|FlowControl|Delay 1.0)
  (Default|PossessPawn _asbp_disconaut))

(fn ConstructionScript)